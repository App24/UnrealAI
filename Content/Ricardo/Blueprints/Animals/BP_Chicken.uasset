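; Chicken animal character driven by an AI blackboard, which the player can interact with while it is outside the coop, lacks line of sight and the player has chicken feed.
; Interacting sets its HasLineOfSight key and rebuilds the player's inventory from only rocks, sticks and plants.
; Its sound replays after short random delays until death, which stops AI logic, flags IsDead, ragdolls the mesh and plays another cue.
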(event `Death_Event`
  (bind _audio (`self.Audio`))
  ;[1 1 1] Take care of killing the chicken
  (`BrainComponent.StopLogic` (`AIController.BrainComponent` (`AIBlueprintHelperLibrary.GetAIController` self)) "")
  (`PrimitiveComponent.SetSimulatePhysics` (`self.Mesh`) true)
  (`PrimitiveComponent.SetCollisionEnabled` (`self.CapsuleComponent`) "NoCollision")
  (`BlackboardComponent.SetValueAsBool` (`AIBlueprintHelperLibrary.GetBlackboard` (`AIBlueprintHelperLibrary.GetAIController` self)) "IsDead" true)
  (`AudioComponent.SetSound` _audio "/Game/FarmAnimalSounds/Animals/Chicken/cue/Chicken_Wings_06_Cue.Chicken_Wings_06_Cue")
  (`AudioComponent.Play` _audio 0.0)
  (`PrimitiveComponent.SetCollisionEnabled` (`self.Mesh`) "QueryAndPhysics"))

(event `self.Audio.OnAudioFinished`
  ;[1 1 1] Play random animal noises
  (if (not (`BlackboardComponent.GetValueAsBool` (`AIBlueprintHelperLibrary.GetBlackboard` (`AIBlueprintHelperLibrary.GetAIController` self)) "IsDead"))
    (`KismetSystemLibrary.Delay` (`KismetMathLibrary.RandomFloatInRange` 0.2 0.35))
    (`AudioComponent.Play` (`self.Audio`) 0.0)))

(event `/Game/Ricardo/Blueprints/BP_IInteractable.OnInteract`
  (`BlackboardComponent.SetValueAsBool` (`AIBlueprintHelperLibrary.GetBlackboard` (`AIBlueprintHelperLibrary.GetAIController` self)) "HasLineOfSight" true)
  (bind _asfirst_person_character (cast `/Game/FirstPersonBP/Blueprints/FirstPersonCharacter` (`GameplayStatics.GetPlayerCharacter` 0)))
  (bind (_rocks _sticks _plants) (break `/Game/Ricardo/Blueprints/BP_PlayerInventory` (`/Game/FirstPersonBP/Blueprints/FirstPersonCharacter.Inventory` _asfirst_person_character)))
  (set `/Game/FirstPersonBP/Blueprints/FirstPersonCharacter.Inventory` (make `/Game/Ricardo/Blueprints/BP_PlayerInventory` _rocks _sticks _plants) _asfirst_person_character))

(event `self.ReceiveBeginPlay`
  (`SceneComponent.SetHiddenInGame` (`self.TextRender`) true false))

(fn `CanInteract`
  (returns (CanPickup :type Boolean))
  (bind _returnvalue (`AIBlueprintHelperLibrary.GetBlackboard` (`AIBlueprintHelperLibrary.GetAIController` self)))
  (bind _asfirst_person_character (cast `/Game/FirstPersonBP/Blueprints/FirstPersonCharacter` (`GameplayStatics.GetPlayerCharacter` 0)))
  (return (and (not (`BlackboardComponent.GetValueAsBool` _returnvalue "InCoop")) (not (`BlackboardComponent.GetValueAsBool` _returnvalue "HasLineOfSight")) (`.HasChickenFeed_9_38F937F746662FBAAFE79BA84C691D59` (break `/Game/Ricardo/Blueprints/BP_PlayerInventory` (`/Game/FirstPersonBP/Blueprints/FirstPersonCharacter.Inventory` _asfirst_person_character))))))

(fn `InteractType`
  (returns (InteractType :type "/Game/Ricardo/Blueprints/EInteractType Enum"))
  (return "NewEnumerator0"))

(fn `LookAtText`
  (returns (Text :type String))
  (return "Chicken"))

(fn `UserConstructionScript`)