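; Base animal Blueprint that plays recurring noises and provides a predator attack against chickens.
; AttackSphere overlaps maintain a list of actors, which Attack scans for chickens to kill when the animal's TooCloseToPlayer and the chicken's HasLineOfSight blackboard keys are true.
; A kill clears the animal's detection keys and updates the predator AI's speed.
; Audio replays after a random delay from GetTimeIntervalBetweenAudio.
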(event `self.AttackSphere.OnComponentBeginOverlap`
  (params (OverlappedComponent :type "PrimitiveComponent Object Reference") (OtherActor :type "Actor Object Reference") (OtherComp :type "PrimitiveComponent Object Reference") (OtherBodyIndex :type Integer) (bFromSweep :type Boolean) (SweepResult :type "HitResult Structure (by ref)"))
  (`KismetArrayLibrary.Array_Add` (`self.OverlapActors`) OtherActor))

(event `self.AttackSphere.OnComponentEndOverlap`
  (params (OverlappedComponent :type "PrimitiveComponent Object Reference") (OtherActor :type "Actor Object Reference") (OtherComp :type "PrimitiveComponent Object Reference") (OtherBodyIndex :type Integer))
  (`KismetArrayLibrary.Array_RemoveItem` (`self.OverlapActors`) OtherActor))

(event `self.Audio.OnAudioFinished`
  ;[1 1 1] Play random animal noises
  (bind (_min _max) (`self.GetTimeIntervalBetweenAudio`))
  (`KismetSystemLibrary.Delay` (`KismetMathLibrary.RandomFloatInRange` _min _max))
  (`AudioComponent.Play` (`self.Audio`) 0.0))

(fn `Attack`
  (bind _returnvalue (`AIBlueprintHelperLibrary.GetBlackboard` (`AIBlueprintHelperLibrary.GetAIController` self)))
  (for _array_element (`self.OverlapActors`)
    (bind _asbp_chicken (cast `/Game/Ricardo/Blueprints/Animals/BP_Chicken` _array_element))
    (if (`BlackboardComponent.GetValueAsBool` (`AIBlueprintHelperLibrary.GetBlackboard` (`AIBlueprintHelperLibrary.GetAIController` self)) "TooCloseToPlayer")
      (if (`BlackboardComponent.GetValueAsBool` (`AIBlueprintHelperLibrary.GetBlackboard` (`AIBlueprintHelperLibrary.GetAIController` _asbp_chicken)) "HasLineOfSight")
        (`/Game/Ricardo/Blueprints/Animals/BP_Chicken.Death_Event` _asbp_chicken)
        (`BlackboardComponent.SetValueAsBool` _returnvalue "HasLineOfSight" false)
        (`BlackboardComponent.SetValueAsBool` _returnvalue "TooCloseToPlayer" false)
        (bind _asbp_base_predator_ai (cast `/Game/Ricardo/Blueprints/AIControllers/BP_BasePredatorAI` (`AIBlueprintHelperLibrary.GetAIController` self)))
        (`/Game/Ricardo/Blueprints/AIControllers/BP_BasePredatorAI.UpdateSpeed` _asbp_base_predator_ai)))))

(fn `GetTimeIntervalBetweenAudio`
  (returns (Min :type "Float (double-precision)") (Max :type "Float (double-precision)"))
  (return 0.2 0.35))

(fn `UserConstructionScript`)