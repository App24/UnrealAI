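; AI controller for BP_Hippo that runs the BT_Hippo behavior tree and manages the hippo's movement speed.
; On BeginPlay it stores its own location as SpawnPosition in the blackboard and caches the original walk speed.
; Perception updates on the player character write HasLineOfSight, then call UpdateSpeed, as does SetSwimState.
; UpdateSpeed gives swimming priority over sight-based speed, setting MaxWalkSpeed for all states; an older speed branch remains unconnected.
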(event `self.ReceiveBeginPlay`
  (`self.RunBehaviorTree` "/Game/Ricardo/BehaviourTrees/BT_Hippo.BT_Hippo")
  (`BlackboardComponent.SetValueAsVector` (`AIBlueprintHelperLibrary.GetBlackboard` null) "SpawnPosition" (`self.K2_GetActorLocation`))
  (bind _charactermovement (`self.GetCharacterMovement`))
  (set `self.OriginalSpeed` (`CharacterMovementComponent.MaxWalkSpeed` _charactermovement)))

(event `self.AIPerception.OnTargetPerceptionUpdated`
  (params (Actor :type "Actor Object Reference") (Stimulus :type "AIStimulus Structure"))
  (cast `/Game/FirstPersonBP/Blueprints/FirstPersonCharacter` Actor)
  (`BlackboardComponent.SetValueAsBool` (`AIBlueprintHelperLibrary.GetBlackboard` null) "HasLineOfSight" (`.bSuccessfullySensed` (break `AIStimulus` Stimulus)))
  (bind _charactermovement (`self.GetCharacterMovement`))
  (`self.UpdateSpeed`))

(fn `GetCharacterMovement`
  (returns (CharacterMovement :type "CharacterMovementComponent Object Reference"))
  (bind _asbp_hippo (cast `/Game/Ricardo/Blueprints/BP_Hippo` (`self.K2_GetPawn`)))
  (return (`Character.CharacterMovement` _asbp_hippo)))

(fn `SetSwimState`
  (params (IsSwimming :type Boolean))
  (set `self.Swimming` IsSwimming)
  (`self.UpdateSpeed`))

(fn `UpdateSpeed`
  (bind _charactermovement (`self.GetCharacterMovement`))
  (if (`self.Swimming`)
    (set `CharacterMovementComponent.MaxWalkSpeed` 250.0 _charactermovement)
    (elif (`BlackboardComponent.GetValueAsBool` (`AIBlueprintHelperLibrary.GetBlackboard` null) "HasLineOfSight")
      (set `CharacterMovementComponent.MaxWalkSpeed` 450.0 _charactermovement)
      (else
        (set `CharacterMovementComponent.MaxWalkSpeed` (`self.OriginalSpeed`) _charactermovement)))))

(fn `UserConstructionScript`)