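; A pickupable rock that the player can collect into their inventory, labelled "Rock" as its look-at text.
; On begin play it gets a random yaw and uniform scale for visual variety.
; Pickup is allowed only while the player character's rock count is under a fixed cap.
; Picking up increments that count, plays a sound, hides the mesh and disables its collision, then destroys the actor when the audio finishes.
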(event `self.ReceiveBeginPlay`
  (`self.K2_AddActorWorldRotation` (`KismetMathLibrary.MakeRotator` 0.0 0.0 (`KismetMathLibrary.RandomFloatInRange` 0.0 360.0)))
  (`self.SetActorScale3D` (`KismetMathLibrary.Conv_DoubleToVector` (`KismetMathLibrary.RandomFloatInRange` 0.6 1.2))))

(event `/Game/Ricardo/Blueprints/BP_IPickupable.OnPickup`
  (bind _staticmeshcomponent (`self.StaticMeshComponent`))
  (bind _asfirst_person_character (cast `/Game/FirstPersonBP/Blueprints/FirstPersonCharacter` (`GameplayStatics.GetPlayerCharacter` 0)))
  (bind (_rocks _sticks _plants _haschickenfeed) (break `/Game/Ricardo/Blueprints/BP_PlayerInventory` (`/Game/FirstPersonBP/Blueprints/FirstPersonCharacter.Inventory` _asfirst_person_character)))
  (set `/Game/FirstPersonBP/Blueprints/FirstPersonCharacter.Inventory` (make `/Game/Ricardo/Blueprints/BP_PlayerInventory` (+ _rocks 1) _sticks _plants _haschickenfeed) _asfirst_person_character)
  (`AudioComponent.Play` (`self.RockPickup`) 0.0)
  (`PrimitiveComponent.SetCollisionEnabled` _staticmeshcomponent "NoCollision")
  (`SceneComponent.SetHiddenInGame` _staticmeshcomponent true false))

(event `self.RockPickup.OnAudioFinished`
  (`self.K2_DestroyActor`))

(fn `CanPickup`
  (returns (CanPickup :type Boolean))
  (bind _asfirst_person_character (cast `/Game/FirstPersonBP/Blueprints/FirstPersonCharacter` (`GameplayStatics.GetPlayerCharacter` 0)))
  (return (< (`.Rocks_2_41BBC99E40F27BAA454C6580D8FA64F8` (break `/Game/Ricardo/Blueprints/BP_PlayerInventory` (`/Game/FirstPersonBP/Blueprints/FirstPersonCharacter.Inventory` _asfirst_person_character))) 5)))

(fn `LookAtText`
  (returns (Text :type String))
  (return "Rock"))

(fn `UserConstructionScript`)