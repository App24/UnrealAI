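; Coop trigger that registers chickens reaching the coop and checks whether the game is finished.
; An overlapping BP_Chicken gets InCoop set on its AI blackboard, with spawn and target locations set to a hardcoded point.
; CheckComplete adds every cooped or dead chicken to ChickensCompleted, which is never reset, and prints a finish message once it reaches the chicken total.
; The trigger then updates that chicken on the player's map widget if it is onscreen.
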(event `self.ReceiveActorBeginOverlap`
  (params (OtherActor :type "Actor Object Reference"))
  (bind _asbp_chicken (cast `/Game/Ricardo/Blueprints/BP_Chicken` OtherActor))
  (bind _returnvalue (`AIBlueprintHelperLibrary.GetBlackboard` (`AIBlueprintHelperLibrary.GetAIController` _asbp_chicken)))
  (`BlackboardComponent.SetValueAsBool` _returnvalue "InCoop" true)
  (`BlackboardComponent.SetValueAsVector` _returnvalue "SpawnLocation" (5910.0 10700.0 170.0))
  (`BlackboardComponent.SetValueAsVector` _returnvalue "TargetLocation" (5910.0 10700.0 170.0))
  (`self.CheckComplete`)
  (bind _asfirst_person_character (cast `/Game/FirstPersonBP/Blueprints/FirstPersonCharacter` (`GameplayStatics.GetPlayerCharacter` 0)))
  (bind _mapwidget (`/Game/FirstPersonBP/Blueprints/FirstPersonCharacter.MapWidget` _asfirst_person_character))
  (`/Engine/EditorBlueprintResources/StandardMacros.IsValid` _mapwidget
    (:`Is Valid`
      (if (`Widget.IsInViewport` _mapwidget)
        (`/Game/Ricardo/Blueprints/Widgets/MapWidget.UpdateChickenUI` _mapwidget _asbp_chicken)))))

(fn `CheckComplete`
  (locals (ChickensCompleted :type Integer))
  (bind _outactors (`GameplayStatics.GetAllActorsOfClass` "/Game/Ricardo/Blueprints/BP_Chicken.BP_Chicken_C"))
  (for _array_element _outactors
    (bind _returnvalue (`AIBlueprintHelperLibrary.GetBlackboard` (`AIBlueprintHelperLibrary.GetAIController` _array_element)))
    (if (or (`BlackboardComponent.GetValueAsBool` _returnvalue "InCoop") (`BlackboardComponent.GetValueAsBool` _returnvalue "IsDead"))
      (set `local.ChickensCompleted` (+ (`local.ChickensCompleted`) 1))))
  (if (>= (`local.ChickensCompleted`) (`KismetArrayLibrary.Array_Length` _outactors))
    (`KismetSystemLibrary.PrintString` "Finished Game")))

(fn `UserConstructionScript`)