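; BP_PlantPickupable is an interactable pickup that adds a plant to the first-person player's inventory.
; It overrides the interaction functions to supply its interact type, show "Plant" as look-at text, and allow pickup only while the player holds fewer than 20 plants.
; Interact rebuilds the inventory struct with the plant count incremented and other fields copied, then calls the parent Interact.
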(fn `CanInteract`
  (returns (CanPickup :type Boolean))
  (bind _asfirst_person_character (cast `/Game/FirstPersonBP/Blueprints/FirstPersonCharacter` (`GameplayStatics.GetPlayerCharacter` 0)))
  (return (< (`.Plants_6_0FC0AD994607A39888113B820D9F50F1` (break `/Game/Ricardo/Blueprints/BP_PlayerInventory` (`/Game/FirstPersonBP/Blueprints/FirstPersonCharacter.Inventory` _asfirst_person_character))) 20)))

(fn `Interact`
  (bind _asfirst_person_character (cast `/Game/FirstPersonBP/Blueprints/FirstPersonCharacter` (`GameplayStatics.GetPlayerCharacter` 0)))
  (bind (_rocks _sticks _plants _haschickenfeed) (break `/Game/Ricardo/Blueprints/BP_PlayerInventory` (`/Game/FirstPersonBP/Blueprints/FirstPersonCharacter.Inventory` _asfirst_person_character)))
  (set `/Game/FirstPersonBP/Blueprints/FirstPersonCharacter.Inventory` (make `/Game/Ricardo/Blueprints/BP_PlayerInventory` _rocks _sticks (+ _plants 1) _haschickenfeed) _asfirst_person_character)
  (`parent.Interact`))

(fn `InteractType`
  (returns (InteractType :type "/Game/Ricardo/Blueprints/EInteractType Enum"))
  (return "NewEnumerator1"))

(fn `LookAtText`
  (returns (Text :type String))
  (return "Plant"))

(fn `UserConstructionScript`)