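; Base Blueprint for pickupable interactables, with an empty Interact function and placeholder defaults for CanInteract, InteractType and LookAtText.
; OnInteract calls Interact, plays the Audio component, then disables collision on the static mesh and hides it.
; The actor destroys itself only when the audio finishes, so the pickup sound is not cut off.
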(event `self.Audio.OnAudioFinished`
  (`self.K2_DestroyActor`))

(event `/Game/Ricardo/Blueprints/BP_IInteractable.OnInteract`
  (bind _staticmesh (`self.StaticMesh`))
  (`self.Interact`)
  (`AudioComponent.Play` (`self.Audio`) 0.0)
  (`PrimitiveComponent.SetCollisionEnabled` _staticmesh "NoCollision")
  (`SceneComponent.SetHiddenInGame` _staticmesh true false))

(fn `CanInteract`
  (returns (CanPickup :type Boolean))
  (return false))

(fn `Interact`)

(fn `InteractType`
  (returns (InteractType :type "/Game/Ricardo/Blueprints/EInteractType Enum"))
  (return "NewEnumerator0"))

(fn `LookAtText`
  (returns (Text :type String))
  (return ""))

(fn `UserConstructionScript`)