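; Base throwable actor that makes noise on impact, both audibly and for AI hearing.
; Its Hit event reports a noise event tagged with the throwable's name, plays an attenuated sound at the impact point, then destroys the actor after a short delay.
; GetThrowableName and GetHitNoise return placeholder values, serving as hooks for child classes to supply the tag and sound.
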(event `self.ReceiveHit`
  (params (MyComp :type "PrimitiveComponent Object Reference") (Other :type "Actor Object Reference") (OtherComp :type "PrimitiveComponent Object Reference") (bSelfMoved :type Boolean) (HitLocation :type "Vector Structure") (HitNormal :type "Vector Structure") (NormalImpulse :type "Vector Structure") (Hit :type "HitResult Structure (by ref)"))
  (bind _name (`self.GetThrowableName`))
  (`AISense_Hearing.ReportNoiseEvent` HitLocation 1.0 self 0.0 _name)
  (bind _sound (`self.GetHitNoise`))
  (`GameplayStatics.PlaySoundAtLocation` _sound HitLocation (struct) 1.0 1.0 0.0 "/Game/Ricardo/ThrowAttenuation.ThrowAttenuation" null null)
  (`KismetSystemLibrary.Delay` 5.0)
  (`self.K2_DestroyActor`))

(fn `GetHitNoise`
  (returns (Sound :type "SoundBase Object Reference"))
  (return null))

(fn `GetThrowableName`
  (returns (Name :type Name))
  (return "None"))

(fn `UserConstructionScript`)