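; BP_ChickenFeed is an interactable pickup that gives the player chicken feed.
; On interact, it rebuilds the first-person character's inventory struct with the feed flag set, keeping rocks, sticks and plants, then plays a grain sound cue.
; Interaction is allowed only while the player lacks feed, and the actor supplies its look-at label and interact type.
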(event `/Game/UserContent/Blueprints/BP_IInteractable.OnInteract`
  (bind _asfirst_person_character (cast `/Game/FirstPersonBP/Blueprints/FirstPersonCharacter` (`GameplayStatics.GetPlayerCharacter` 0)))
  (bind (_rocks _sticks _plants) (break `/Game/UserContent/Blueprints/BP_PlayerInventory` (`/Game/FirstPersonBP/Blueprints/FirstPersonCharacter.Inventory` _asfirst_person_character)))
  (set `/Game/FirstPersonBP/Blueprints/FirstPersonCharacter.Inventory` (make `/Game/UserContent/Blueprints/BP_PlayerInventory` _rocks _sticks _plants true) _asfirst_person_character)
  (`AudioComponent.Play` (`self.Grains_10_Cue`) 0.0))

(fn `CanInteract`
  (returns (CanPickup :type Boolean))
  (bind _asfirst_person_character (cast `/Game/FirstPersonBP/Blueprints/FirstPersonCharacter` (`GameplayStatics.GetPlayerCharacter` 0)))
  (return (not (`.HasChickenFeed_9_38F937F746662FBAAFE79BA84C691D59` (break `/Game/UserContent/Blueprints/BP_PlayerInventory` (`/Game/FirstPersonBP/Blueprints/FirstPersonCharacter.Inventory` _asfirst_person_character))))))

(fn `InteractType`
  (returns (InteractType :type "/Game/UserContent/Blueprints/EInteractType Enum"))
  (return "NewEnumerator0"))

(fn `LookAtText`
  (returns (Text :type String))
  (return "Chicken Feed"))

(fn `UserConstructionScript`)