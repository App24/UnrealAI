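; Base AI controller for predators that hunt chickens and can be distracted by throwables, with stub getters for behavior tree, chase speed and distraction tags.
; BeginPlay runs the tree and stores spawn position and original walk speed.
; Perception updates feed ChaseChicken, which sets blackboard target, sight and speed, falling back to BecomeDistracted for a timed diversion toward tagged stimuli.
; The ChasePlayer branch is disconnected.
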(event `self.ReceiveBeginPlay`
  (bind _behaviourtree (`self.GetBehaviourTree`))
  (`self.RunBehaviorTree` _behaviourtree)
  (`BlackboardComponent.SetValueAsVector` (`AIBlueprintHelperLibrary.GetBlackboard` null) "SpawnPosition" (`self.K2_GetActorLocation`))
  (bind _charactermovement (`self.GetCharacterMovement`))
  (set `self.OriginalSpeed` (`CharacterMovementComponent.MaxWalkSpeed` _charactermovement)))

(event `self.AIPerception.OnTargetPerceptionUpdated`
  (params (Actor :type "Actor Object Reference") (Stimulus :type "AIStimulus Structure"))
  (`self.ChaseChicken` Actor Stimulus
    (:`Cast Failed`
      (`self.BecomeDistracted` Actor Stimulus))))

(fn `GetBehaviourTree`
  (returns (BehaviourTree :type "BehaviorTree Object Reference"))
  (return null))

(fn `GetCharacterMovement`
  (returns (CharacterMovement :type "CharacterMovementComponent Object Reference"))
  (bind _ascharacter (cast `Character` (`self.K2_GetPawn`)))
  (return (`Character.CharacterMovement` _ascharacter)))

(fn `GetChaseSpeed`
  (returns (Speed :type "Float (double-precision)"))
  (return 0.0))

(fn `GetDistractedTags`
  (returns (Names :type "Array of Name"))
  (return))

(fn `SetSpeed`
  (params (Speed :type "Float (double-precision)"))
  (bind _charactermovement (`self.GetCharacterMovement`))
  (set `CharacterMovementComponent.MaxWalkSpeed` Speed _charactermovement))

(fn `UpdateSpeed`
  (bind _charactermovement (`self.GetCharacterMovement`))
  (if (`BlackboardComponent.GetValueAsBool` (`AIBlueprintHelperLibrary.GetBlackboard` null) "HasLineOfSight")
    (bind _speed (`self.GetChaseSpeed`))
    (set `CharacterMovementComponent.MaxWalkSpeed` _speed _charactermovement)
    (else
      (set `CharacterMovementComponent.MaxWalkSpeed` (`self.OriginalSpeed`) _charactermovement))))

(fn `UserConstructionScript`)