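; BP_HippoAI is the AI controller for the hippo animal, overriding hooks from a parent AI class.
; It supplies the hippo behavior tree, its chase speed and "Plant" as the tag that can distract it.
; SetSwimState records whether the hippo is swimming and refreshes movement speed, which uses a fixed swim speed in water and otherwise defers to the parent's speed logic.
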(fn `GetBehaviourTree`
  (returns (BehaviourTree :type "BehaviorTree Object Reference"))
  (return "/Game/UserContent/BehaviourTrees/BT_Hippo.BT_Hippo"))

(fn `GetChaseSpeed`
  (returns (Speed :type "Float (double-precision)"))
  (return 450.0))

(fn `GetDistractedTags`
  (returns (Names :type "Array of Name"))
  (return (`|MakeArray` "Plant" :!type "Name")))

(fn `SetSwimState`
  (params (IsSwimming :type Boolean))
  (set `self.Swimming` IsSwimming)
  (`self.UpdateSpeed`))

(fn `UpdateSpeed`
  (if (`self.Swimming`)
    (`self.SetSpeed` 250.0)
    (else
      (`parent.UpdateSpeed`))))

(fn `UserConstructionScript`)