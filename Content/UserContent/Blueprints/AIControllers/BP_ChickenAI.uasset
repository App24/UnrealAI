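; BP_ChickenAI is the AI controller for chicken pawns, running the BT_Chicken behavior tree and adjusting walk speed by distance to the target.
; Each tick it measures the distance from the pawn to the blackboard's TargetLocation and switches to a fixed chase speed when far away.
; A Chasing flag adds hysteresis, holding that speed until the chicken gets much closer, then restoring the original speed cached at BeginPlay.
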(event `self.ReceiveBeginPlay`
  (`self.RunBehaviorTree` "/Game/UserContent/BehaviourTrees/BT_Chicken.BT_Chicken")
  (bind _charactermovement (`self.GetCharacterMovement`))
  (set `self.OriginalSpeed` (`CharacterMovementComponent.MaxWalkSpeed` _charactermovement)))

(event `self.ReceiveTick`
  (params (DeltaSeconds :type "Float (single-precision)"))
  (bind _returnvalue (`KismetMathLibrary.Vector_Distance` (`BlackboardComponent.GetValueAsVector` (`AIBlueprintHelperLibrary.GetBlackboard` null) "TargetLocation") (`self.K2_GetActorLocation` (`self.K2_GetPawn`))))
  ;[1 1 1] Change the chicken's speed depending how far away they are from their target location
  (bind _charactermovement (`self.GetCharacterMovement`))
  (if (> _returnvalue 600.0)
    (set `CharacterMovementComponent.MaxWalkSpeed` 300.0 _charactermovement)
    (set `self.Chasing` true)
    (elif (`self.Chasing`)
      (if (not (> _returnvalue 300.0))
        (set `self.Chasing` false))
      (else
        (set `CharacterMovementComponent.MaxWalkSpeed` (`self.OriginalSpeed`) _charactermovement)))))

(fn `GetCharacterMovement`
  (returns (CharacterMovement :type "CharacterMovementComponent Object Reference"))
  (bind _asbp_chicken (cast `/Game/UserContent/Blueprints/Animals/BP_Chicken` (`self.K2_GetPawn`)))
  (return (`Character.CharacterMovement` _asbp_chicken)))

(fn `UserConstructionScript`)