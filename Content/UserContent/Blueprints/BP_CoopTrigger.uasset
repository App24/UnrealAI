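; BP_CoopTrigger is a trigger volume that registers chickens herded into the coop.
; On overlap with a BP_Chicken, it sets that chicken's AI blackboard to in-coop, clears line of sight to stop following, and pins spawn and target locations to a hardcoded coop point.
; It then calls CheckComplete on the player character and updates the map widget's chicken UI if that widget is on screen.
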(event `self.ReceiveActorBeginOverlap`
  (params (OtherActor :type "Actor Object Reference"))
  (bind _asbp_chicken (cast `/Game/UserContent/Blueprints/Animals/BP_Chicken` OtherActor))
  (bind _returnvalue (`AIBlueprintHelperLibrary.GetBlackboard` (`AIBlueprintHelperLibrary.GetAIController` _asbp_chicken)))
  ;[1 1 1] Put chicken in coop
  (`BlackboardComponent.SetValueAsBool` _returnvalue "InCoop" true)
  ;[1 1 1] Stop chicken from following player
  (`BlackboardComponent.SetValueAsBool` _returnvalue "HasLineOfSight" false)
  ;[1 1 1] Ensure chicken is confined to the bounds of the coop
  (`BlackboardComponent.SetValueAsVector` _returnvalue "SpawnLocation" (5910.0 10700.0 170.0))
  (`BlackboardComponent.SetValueAsVector` _returnvalue "TargetLocation" (5910.0 10700.0 170.0))
  (bind _asfirst_person_character (cast `/Game/FirstPersonBP/Blueprints/FirstPersonCharacter` (`GameplayStatics.GetPlayerCharacter` 0)))
  (`/Game/FirstPersonBP/Blueprints/FirstPersonCharacter.CheckComplete` _asfirst_person_character)
  (bind _mapwidget (`/Game/FirstPersonBP/Blueprints/FirstPersonCharacter.MapWidget` _asfirst_person_character))
  (`/Engine/EditorBlueprintResources/StandardMacros.IsValid` _mapwidget
    (:`Is Valid`
      (if (`Widget.IsInViewport` _mapwidget)
        (`/Game/UserContent/Blueprints/Widgets/MapWidget.UpdateChickenUI` _mapwidget _asbp_chicken)))))

(fn `UserConstructionScript`)